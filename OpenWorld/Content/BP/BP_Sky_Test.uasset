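; Sky sphere actor running a day/night cycle with moving sun, clouds and stars.
; Tick advances Time by a fixed, frame-rate-dependent step, pitching the directional light over a 24-hour cycle.
; UpdateSkyM derives SunHeight from that pitch and feeds a dynamic sky material created at construction.
; With ColorsDeterminedBySunPosition on, color curves also tint the sun, skylight and height fog; otherwise manual sky colors apply.
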(event EventBeginPlay)

(event Collision|EventActorBeginOverlap
  (params (OtherActor :type Actor%20Object%20Reference)))

(event EventTick
  (params (DeltaSeconds :type Float%20%28single-precision%29))
  (Variables|Default|SetTime (+ (Variables|Default|GetTime) 0.005))
  (CallFunction|UpdateTime))

(event EventUpdateSky
  (Utilities|UpdateSkyM))

(fn ConstructionScript
  (CallFunction|UpdateTime)
  (bind _returnvalue (Rendering|Material|CreateDynamicMaterialInstance (Variables|Default|GetSkySphereMesh) 0 "/Game/Materials/M_Sky_Panning_Clouds_WithMoon_Inst.M_Sky_Panning_Clouds_WithMoon_Inst" "None" :!class /Script/Engine.PrimitiveComponent))
  (Variables|Default|SetSky%20material _returnvalue)
  (if (Variables|Default|GetRefresh%20material) ; Updating bool in details panel causes construction script to run again
    _
    (else
      _))
  (Variables|Default|SetRefresh%20material false)
  (CallFunction|RefreshMaterial))

(fn UpdateTime
  (Transformation|SetActorRotation (Variables|Default|GetDirectional%20light%20actor) (Math|Rotator|MakeRotator 0.0 (+ (* (/ (Math|Float|%(Float) (Variables|Default|GetTime) 24.0) 24.0) 3.6e+02) 9e+01) 0.0))
  (Variables|Default|SetRefresh%20material true)
  (CallFunction|UpdateSky))